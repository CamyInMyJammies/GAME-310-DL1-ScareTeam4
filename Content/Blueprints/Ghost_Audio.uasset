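; Ghost audio Blueprint that plays a ghost sound through its Audio component.
; On BeginPlay it assigns the sound, attenuation, concurrency set and volume from its variables, then activates the component.
; Playback starts at a random point within the sound's duration, so separate instances do not play in sync.
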(event `self.ReceiveBeginPlay`
  (bind _audio (`self.Audio`))
  (`AudioComponent.SetSound` _audio (`self.Ghost Sounds`))
  (set `AudioComponent.AttenuationSettings` (`self.Ghost Attenuation`) _audio)
  (set `AudioComponent.ConcurrencySet` (`|MakeSet` (`self.Ghost Concurrency`)) _audio)
  (`AudioComponent.SetVolumeMultiplier` _audio (`self.Ghost Volume`))
  (`ActorComponent.SetActive` _audio true false)
  (`AudioComponent.Play` _audio (* (`KismetMathLibrary.RandomFloatInRange` 0.0 1.0) (`SoundBase.Duration` (`self.Ghost Sounds`)))))

(fn `UserConstructionScript`)